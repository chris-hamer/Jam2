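; AggroGroup is a trigger actor that keeps a group of enemies dormant until the player character, a JamCharacter, overlaps it.
; On BeginPlay it sets Inactive on every valid entry in its Enemies array.
; The first JamCharacter overlap clears that flag on all valid entries, and a DoOnce keeps later overlaps from repeating the wake-up.
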(event Collision|EventActorBeginOverlap
  (params (OtherActor :type Actor%20Object%20Reference))
  (Utilities|Casting|CastToJamCharacter OtherActor)
  (Utilities|FlowControl|DoOnce false
    (:Completed
      (for _array_element (Variables|Default|GetEnemies)
        (Utilities|IsValid _array_element
          (:Is%20Valid
            (Variables|/Game/Blueprints/Enemy/Enemy_Troll/BigGuy.BigGuy_C|SetInactive _array_element false)))))))

(event EventTick
  (params (DeltaSeconds :type Float%20%28single-precision%29)))

(event EventBeginPlay
  (for _array_element (Variables|Default|GetEnemies)
    (Utilities|IsValid _array_element
      (:Is%20Valid
        (Variables|/Game/Blueprints/Enemy/Enemy_Troll/BigGuy.BigGuy_C|SetInactive _array_element true)))))

(fn ConstructionScript)