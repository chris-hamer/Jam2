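; Attack state for the player's state machine, performing a sword swing.
; On enter, it turns the player toward movement input, or keeps forward facing without input, plays the sword montage sped up and ends hit stop.
; Each tick halts movement and calls stamina regeneration.
; Dodge input switches state if stamina can be consumed, while an End input switches to another state.
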(event EventEnter
  (params (PlayerCharacter :type Jam%20Character%20Object%20Reference))
  (bind _output_get (Variables|Default|SetPlayer PlayerCharacter))
  (Transformation|SetActorRotation _output_get (Math|Conversions|RotationFromXVector (select (Math|Float|NearlyEqual(Float) (Math|Vector|VectorLength (Variables|/Game/Blueprints/JamCharacter.JamCharacter_C|GetAdjustedMovementInput _output_get)) 0.0 0.001) (Transformation|GetActorForwardVector _output_get) (Variables|/Game/Blueprints/JamCharacter.JamCharacter_C|GetAdjustedMovementInput _output_get))))
  (Animation|Montage|MontagePlay (Components|SkeletalMesh|GetAnimInstance (Variables|/Script/Engine.Character|GetMesh (Variables|Default|GetPlayer))) "/Game/Models/Animations/HeroTPP_sword1_Montage.HeroTPP_sword1_Montage" 2.5 "MontageLength" 0.0)
  (Default|EndHitStop (Variables|Default|GetPlayer)))

(event EventTickState
  (params (PlayerCharacter :type Jam%20Character%20Object%20Reference))
  (Components|Movement|StopMovementImmediately (Variables|/Script/Engine.Character|GetCharacterMovement (Variables|Default|GetPlayer)))
  (Default|RegenStamina (Variables|Default|GetPlayer) true))

(event EventInputEvent
  (params (PlayerCharacter :type Jam%20Character%20Object%20Reference) (Input :type Inputs%20Enum :default "NewEnumerator0"))
  (switch Utilities|FlowControl|Switch|SwitchonInputs Input
    (:NewEnumerator1
      (bind _hadenough (Default|ConsumeStamina (Variables|Default|GetPlayer)))
      (if _hadenough
        (Default|SetState (Variables|Default|GetPlayer) "NewEnumerator1")))
    (:NewEnumerator2
      (Default|SetState (Variables|Default|GetPlayer) "NewEnumerator0"))))