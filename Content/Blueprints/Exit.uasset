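; Exit actor that stays hidden until every actor or object in its Things array is gone, then shows a widget when the player reaches it.
; BeginPlay hides the Cube and disables its collision.
; Tick counts valid Things entries each frame and, at zero, makes the Cube visible with full collision.
; An actor overlap that casts to JamCharacter creates a DIDTHEDO widget and adds it to the viewport.
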(event EventBeginPlay
  (Rendering|SetVisibility (Variables|Default|GetCube) false false)
  (Collision|SetCollisionEnabled (Variables|Default|GetCube) "NoCollision"))

(event Collision|EventActorBeginOverlap
  (params (OtherActor :type Actor%20Object%20Reference))
  (Utilities|Casting|CastToJamCharacter OtherActor)
  (bind _returnvalue (UserInterface|CreateWidget "/Game/Blueprints/HUD/DIDTHEDO.DIDTHEDO_C"))
  (UserInterface|Viewport|AddtoViewport _returnvalue 0))

(event EventTick
  (params (DeltaSeconds :type Float%20%28single-precision%29))
  (Variables|Default|Setv 0)
  (for _array_element (Variables|Default|Getthings)
    (Utilities|IsValid _array_element
      (:Is%20Valid
        (Math|Integer|IncrementInt (Variables|Default|Getv)))))
  (if (== (Variables|Default|Getv) 0)
    (Rendering|SetVisibility (Variables|Default|GetCube) true false)
    (Collision|SetCollisionEnabled (Variables|Default|GetCube) "QueryAndPhysics")))

(fn ConstructionScript)