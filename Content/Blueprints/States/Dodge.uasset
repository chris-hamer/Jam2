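; Player dodge state that rolls the character along its movement input, or opposite its facing when there is none.
; Enter plays the roll montage, switches characters, ignores Pawn collision and ends attacks and hit stop.
; TickState drives movement and clamps horizontal velocity to a speed that decays quadratically with montage progress, preserving vertical velocity.
; Exit restores walk speed and acceleration; End input changes state and stops the montage.
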(event EventEnter
  (params (PlayerCharacter :type Jam%20Character%20Object%20Reference))
  (bind _output_get (Variables|Default|SetPlayer PlayerCharacter))
  (bind _output_get_2 (Variables|Default|SetDodgeDirection (select (Math|Float|NearlyEqual(Float) (Math|Vector|VectorLength (Variables|/Game/Blueprints/JamCharacter.JamCharacter_C|GetAdjustedMovementInput _output_get)) 0.0 0.001) (* (Transformation|GetActorForwardVector _output_get) -1.0) (Variables|/Game/Blueprints/JamCharacter.JamCharacter_C|GetAdjustedMovementInput _output_get))))
  (Transformation|SetActorRotation _output_get (Math|Conversions|RotationFromXVector _output_get_2))
  (bind _output_get_3 (Variables|/Script/Engine.CharacterMovementComponent|SetMaxWalkSpeed (Variables|/Script/Engine.Character|GetCharacterMovement (Variables|Default|GetPlayer)) (Variables|/Game/Blueprints/JamCharacter.JamCharacter_C|GetDodgeSpeed (Variables|Default|GetPlayer))))
  (Variables|/Script/Engine.CharacterMovementComponent|SetMaxAcceleration (Variables|/Script/Engine.Character|GetCharacterMovement (Variables|Default|GetPlayer)) 5e+04)
  (Variables|Default|SetCurrentDodgeSpeed _output_get_3)
  (Animation|Montage|MontagePlay (Components|SkeletalMesh|GetAnimInstance (Variables|/Script/Engine.Character|GetMesh (Variables|Default|GetPlayer))) "/Game/Models/Animations/HeroTPP_roll_Montage.HeroTPP_roll_Montage" 1.0 "MontageLength" 0.0)
  (Default|SwitchCharacters (Variables|Default|GetPlayer))
  (Collision|SetCollisionResponsetoChannel (Variables|/Script/Engine.Character|GetCapsuleComponent (Variables|Default|GetPlayer)) "ECC_Pawn" "ECR_Ignore")
  (Default|AttackEnd (Variables|Default|GetPlayer))
  (Default|EndHitStop (Variables|Default|GetPlayer)))

(event EventExit
  (params (PlayerCharacter :type Jam%20Character%20Object%20Reference))
  (Variables|/Script/Engine.CharacterMovementComponent|SetMaxWalkSpeed (Variables|/Script/Engine.Character|GetCharacterMovement (Variables|Default|GetPlayer)) 6e+02)
  (Variables|/Script/Engine.CharacterMovementComponent|SetMaxAcceleration (Variables|/Script/Engine.Character|GetCharacterMovement (Variables|Default|GetPlayer)) 2048.0))

(event EventTickState
  (params (PlayerCharacter :type Jam%20Character%20Object%20Reference))
  (bind _player (Variables|Default|GetPlayer))
  (bind _player_2 (Variables|Default|GetPlayer))
  (bind _charactermovement (Variables|/Script/Engine.Character|GetCharacterMovement _player_2))
  (bind _mesh (Variables|/Script/Engine.Character|GetMesh _player))
  (bind _returnvalue (Components|SkeletalMesh|GetAnimInstance _mesh))
  (bind _returnvalue_2 (Animation|Montage|GetCurrentActiveMontage _returnvalue))
  (Class|PawnMovementComponent|AddInputVector (Pawn|GetMovementComponent (Variables|Default|GetPlayer)) (Variables|Default|GetDodgeDirection) false)
  (Default|RegenStamina (Variables|Default|GetPlayer) false)
  (Utilities|IsValid _returnvalue_2
    (:Is%20Valid
      (bind _output_get (Variables|Default|SetCurrentDodgeSpeed (* (Variables|/Game/Blueprints/JamCharacter.JamCharacter_C|GetDodgeSpeed (Variables|Default|GetPlayer)) (Math|Float|Power (- 1.0 (/ (* (Animation|Montage|MontageGetPosition _returnvalue _returnvalue_2) (Class|AnimInstance|MontageGetPlayRate _returnvalue _returnvalue_2)) (Variables|/Script/Engine.AnimSequenceBase|GetSequenceLength _returnvalue_2))) 2.0))))
      (bind _output_get_2 (Variables|/Script/Engine.CharacterMovementComponent|SetMaxWalkSpeed _charactermovement _output_get))
      (Variables|/Script/Engine.MovementComponent|SetVelocity _charactermovement (+ (Math|Vector|ClampVectorSize (Math|Vector|ProjectVectorontoPlane (Variables|/Script/Engine.MovementComponent|GetVelocity _charactermovement) "0, 0,1.000000") 0.0 _output_get_2) (Math|Vector|ProjectVectorontoVector (Variables|/Script/Engine.MovementComponent|GetVelocity _charactermovement) "0, 0,1.000000"))))))

(event EventInputEvent
  (params (PlayerCharacter :type Jam%20Character%20Object%20Reference) (Input :type Inputs%20Enum :default "NewEnumerator0"))
  (switch Utilities|FlowControl|Switch|SwitchonInputs Input
    (:NewEnumerator2
      (Default|SetState (Variables|Default|GetPlayer) "NewEnumerator0")
      (Animation|Montage|MontageStop (Components|SkeletalMesh|GetAnimInstance (Variables|/Script/Engine.Character|GetMesh (Variables|Default|GetPlayer))) 0.0 "/Game/Models/Animations/HeroTPP_roll_Montage.HeroTPP_roll_Montage"))))